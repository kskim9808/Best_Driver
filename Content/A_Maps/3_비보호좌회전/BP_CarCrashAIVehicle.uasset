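; AI vehicle for the unprotected left-turn map that stages a car crash and moves on to the control center level.
; When its box overlaps a BP_CarCrashAIOtherVehicle, both cars stop, and a Cnt counter limits how often the crash sequence runs.
; The sequence fades the camera toward translucent red, puts an X widget on the traffic-obstruction CCTV found at BeginPlay, then slows global time before opening 33_관제센터.
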(event OnComponentBeginOverlap(boxComp)
  (params (OverlappedComponent :type Primitive%20Component%20Object%20Reference) (OtherActor :type Actor%20Object%20Reference) (OtherComp :type Primitive%20Component%20Object%20Reference) (OtherBodyIndex :type Integer) (bFromSweep :type Boolean) (SweepResult :type Hit%20Result%20Structure%20%28by%20ref%29))
  (bind _asbp_car_crash_aiother_vehicle (Utilities|Casting|CastToBP_CarCrashAIOtherVehicle OtherActor))
  (Class|CarCrashAIVehicle|Stop _asbp_car_crash_aiother_vehicle)
  (Class|CarCrashAIVehicle|Stop)
  (if (>= (Variables|Default|Getcnt) 1)
    (Variables|Default|Setcnt (- (Variables|Default|Getcnt) 1))
    (CameraFades|StartCameraFade (Game|GetPlayerCameraManager 0) 0.0 0.3 3.0 "(R=1.000000,G=0.000000,B=0.000000,A=1.000000)" true false)
    (Utilities|FlowControl|Delay 2.0)
    (bind _returnvalue (UserInterface|CreateWidget "/Game/A_Maps/3_비보호좌회전/위젯/x.x_C"))
    (UserInterface|SetWidget (Variables|/Game/A_Maps/3_비보호좌회전/3-2_통행방해cctv.3-2_통행방해cctv_C|GetWidget (Variables|Default|Get3-2_cctv)) _returnvalue)
    (Utilities|Time|SetGlobalTimeDilation 0.1)
    (Utilities|FlowControl|Delay 0.5)
    (Game|OpenLevel(byObjectReference) "/Game/A_Maps/3_비보호좌회전/3-3_관제센터.3-3_관제센터")))

(event EventBeginPlay
  (bind _returnvalue (Actor|GetActorOfClass "/Game/A_Maps/3_비보호좌회전/3-2_통행방해cctv.3-2_통행방해cctv_C"))
  (Variables|Default|Set3-2_cctv _returnvalue))

(event Collision|EventActorBeginOverlap
  (params (OtherActor :type Actor%20Object%20Reference)))

(event EventTick
  (params (DeltaSeconds :type Float%20%28single-precision%29)))

(fn ConstructionScript)