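; Stage 1 traffic signal that starts a looping light cycle once the player enters its trigger box, gated by the Isfinish flag.
; Four near-identical macros, Seq1 to Seq4, run in a chain, with Seq4 looping back to Seq1.
; Each reads its Sequence struct to set red, yellow, green-left-turn and green body materials and matching component visibility, then delays for that step's duration, or bypasses the step when unused.
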(event OnComponentBeginOverlap(boxComp)
  (params (OverlappedComponent :type Primitive%20Component%20Object%20Reference) (OtherActor :type Actor%20Object%20Reference) (OtherComp :type Primitive%20Component%20Object%20Reference) (OtherBodyIndex :type Integer) (bFromSweep :type Boolean) (SweepResult :type Hit%20Result%20Structure%20%28by%20ref%29))
  (Utilities|Casting|CastTo2_BP_Stage1_PLAYER OtherActor)
  (if (Variables|Default|GetIsfinish)
    (Variables|Default|SetIsfinish false)
    (|Seq1 :!label _label
      (:then
        _)
      (:Not%20use
        _))
    (|Seq2
      (:then
        _)
      (:Not%20Use
        _))
    (|Seq3
      (:then
        _)
      (:Not%20Use
        _))
    (|Seq4
      (:then
        (goto _label))
      (:Not%20Use
        (goto _label)))))

(event EventBeginPlay
  (Utilities|FlowControl|Sequence
    (:then_0
      (Rendering|Material|SetMaterial (Variables|Default|GetbodyMesh) 1 "/Game/roadtrafficlights/Materials/RoadSignal/M_Road_Signal_Red_OFF.M_Road_Signal_Red_OFF")
      (Rendering|SetVisibility (Variables|Default|GetredRight) true false))
    (:then_1
      (Rendering|Material|SetMaterial (Variables|Default|GetbodyMesh) 2 "/Game/roadtrafficlights/Materials/RoadSignal/M_Road_Signal_Yellow_OFF.M_Road_Signal_Yellow_OFF")
      (Rendering|SetVisibility (Variables|Default|GetyellowRight) true false))
    (:then_2
      (Rendering|Material|SetMaterial (Variables|Default|GetbodyMesh) 3 "/Game/roadtrafficlights/Materials/RoadSignal/M_Road_Signal_Green_Lturn_ON.M_Road_Signal_Green_Lturn_ON")
      (Rendering|SetVisibility (Variables|Default|GetgreenLTurnRight) false false))
    (:then_3
      (Rendering|Material|SetMaterial (Variables|Default|GetbodyMesh) 3 "/Game/roadtrafficlights/Materials/RoadSignal/M_Road_Signal_Green_ON.M_Road_Signal_Green_ON")
      (Rendering|SetVisibility (Variables|Default|GetgreenRight) false false))))

(fn ConstructionScript)