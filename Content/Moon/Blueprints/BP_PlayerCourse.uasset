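; BP_PlayerCourse is a spline-driven actor that builds a course out of spline meshes, with no runtime logic.
; The construction script divides the spline into equal segments of at most about 500 units and adds a spline mesh component for each.
; Each segment takes its endpoints and length-clamped tangents from the spline, and the spline point's Y scale, halved, sizes both cross-section axes.
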(event EventBeginPlay)

(event Collision|EventActorBeginOverlap
  (params (OtherActor :type Actor%20Object%20Reference)))

(event EventTick
  (params (DeltaSeconds :type Float%20%28single-precision%29)))

(fn ConstructionScript
  (bind _returnvalue (Math|Float|Clamp(Float) 5e+02 5e+01 1e+06))
  (bind _spline (Variables|Default|GetSpline))
  (bind _spline_2 (Variables|Default|GetSpline))
  (bind _spline_3 (Variables|Default|GetSpline))
  (bind _returnvalue_2 (Spline|GetSplineLength _spline_3))
  (bind _returnvalue_3 (/ _returnvalue_2 _returnvalue))
  (bind _returnvalue_4 (Math|Float|Truncate _returnvalue_3))
  (bind _output_get (Variables|Default|SetLast%20Index _returnvalue_4))
  (Variables|Default|SetSegment%20Length%20Corrected (/ (Spline|GetSplineLength (Variables|Default|GetSpline)) (Math|Conversions|ToFloat(Integer) (+ _returnvalue_4 1))))
  (for _index (range 0 _output_get)
    (bind _returnvalue_5 (AddComponent|AddSplineMeshComponent false))
    (SplineMesh|SetForwardAxis _returnvalue_5 "X" true)
    (SplineMesh|SetStartandEnd _returnvalue_5 (Spline|GetLocationatDistanceAlongSpline _spline (* (Variables|Default|GetSegment%20Length%20Corrected) (Math|Conversions|ToFloat(Integer) _index)) "Local") (Math|Vector|ClampVectorSize (Spline|GetTangentatDistanceAlongSpline _spline (* (Variables|Default|GetSegment%20Length%20Corrected) (Math|Conversions|ToFloat(Integer) _index)) "Local") 0.0 (Variables|Default|GetSegment%20Length%20Corrected)) (Spline|GetLocationatDistanceAlongSpline _spline_2 (* (Variables|Default|GetSegment%20Length%20Corrected) (Math|Conversions|ToFloat(Integer) (+ _index 1))) "Local") (Math|Vector|ClampVectorSize (Spline|GetTangentatDistanceAlongSpline _spline_2 (* (Variables|Default|GetSegment%20Length%20Corrected) (Math|Conversions|ToFloat(Integer) (+ _index 1))) "Local") 0.0 (Variables|Default|GetSegment%20Length%20Corrected)) true :!class /Script/Engine.SplineMeshComponent)
    (SplineMesh|SetStartScale _returnvalue_5 (Math|Vector2D|MakeVector2D (* (.y (Class|SplineComponent|GetScaleatDistanceAlongSpline _spline (* (Variables|Default|GetSegment%20Length%20Corrected) (Math|Conversions|ToFloat(Integer) _index)))) 0.5) (* 1.0 (* (.y (Class|SplineComponent|GetScaleatDistanceAlongSpline _spline (* (Variables|Default|GetSegment%20Length%20Corrected) (Math|Conversions|ToFloat(Integer) _index)))) 0.5))) true :!class /Script/Engine.SplineMeshComponent)
    (SplineMesh|SetEndScale _returnvalue_5 (Math|Vector2D|MakeVector2D (* (.y (Class|SplineComponent|GetScaleatDistanceAlongSpline _spline_2 (* (Variables|Default|GetSegment%20Length%20Corrected) (Math|Conversions|ToFloat(Integer) (+ _index 1))))) 0.5) (* 1.0 (* (.y (Class|SplineComponent|GetScaleatDistanceAlongSpline _spline_2 (* (Variables|Default|GetSegment%20Length%20Corrected) (Math|Conversions|ToFloat(Integer) (+ _index 1))))) 0.5))) true :!class /Script/Engine.SplineMeshComponent)))