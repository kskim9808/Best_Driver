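; Spline-driven wire actor that builds a deformed mesh along an editable spline, by its name for cables in the Korean street corner environment.
; The construction script adds one spline mesh component per segment between neighboring spline points, using the Mesh and ForwardAxis variables.
; Each segment attaches to the spline and takes its start and end positions and tangents from the two points in local space, so it follows the curve.
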(fn ConstructionScript
  (bind _spline (Variables|Default|GetSpline))
  (for _index (range 0 (- (Spline|GetNumberOfSplinePoints _spline) 2))
    (bind _returnvalue (AddComponent|AddSplineMeshComponent false (Math|Transform|MakeTransform "0, 0, 0")))
    (Components|StaticMesh|SetStaticMesh _returnvalue (Variables|Default|GetMesh))
    (SplineMesh|SetForwardAxis _returnvalue (Variables|Default|GetForwardAxis) true)
    (Transformation|AttachComponentToComponent _returnvalue _spline "None" "KeepRelative" "KeepRelative" "KeepRelative" true)
    (SplineMesh|SetStartandEnd _returnvalue (.Location (Spline|GetLocationandTangentatSplinePoint _spline _index "Local")) (.Tangent (Spline|GetLocationandTangentatSplinePoint _spline _index "Local")) (.Location (Spline|GetLocationandTangentatSplinePoint _spline (+ _index 1) "Local")) (.Tangent (Spline|GetLocationandTangentatSplinePoint _spline (+ _index 1) "Local")) true :!class /Script/Engine.SplineMeshComponent)))