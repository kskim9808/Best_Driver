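; BP_OfficeCable is an office cable prop built entirely in the construction script from an editable spline.
; Ends with a valid socket actor snap their spline point and tangent to that socket, adjusted by plug type and flip.
; Spline mesh segments follow the curve, sharing a dynamic material for width and color, with computed up vectors.
; Tinted plug meshes cap both ends, using plugged or loose variants.
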(event EventBeginPlay)

(event Collision|EventActorBeginOverlap
  (params (OtherActor :type Actor%20Object%20Reference)))

(event EventTick
  (params (DeltaSeconds :type Float%20%28single-precision%29)))

(fn ConstructionScript
  (bind _spline (Variables|Default|GetSpline))
  (bind _spline_2 (Variables|Default|GetSpline))
  (bind _returnvalue (Rendering|Material|CreateDynamicMaterialInstance "/Game/BasicOffice/Materials/Cable/M_Cable.M_Cable" :!class /Script/Engine.KismetMaterialLibrary))
  (bind _output_get (Variables|Default|SetDynamicMaterialInstance _returnvalue))
  (Rendering|Material|SetScalarParameterValue _output_get "Cable Width" (Variables|Cable|GetWidth) :!class /Script/Engine.MaterialInstanceDynamic)
  (Rendering|Material|SetVectorParameterValue (Variables|Default|GetDynamicMaterialInstance) "Color" (Variables|Cable|GetColor) :!class /Script/Engine.MaterialInstanceDynamic)
  (Utilities|FlowControl|Sequence
    (:then_0
      (CallFunction|PlugtoSocket false)
      (CallFunction|PlugtoSocket true))
    (:then_1
      (for _index (range 0 (- (Spline|GetNumberOfSplinePoints (Variables|Default|GetSpline)) 2))
        (bind _returnvalue_2 (AddComponent|AddSplineMeshComponent false))
        (bind _output_get_2 (LocalVariables|SetLocal%20SMesh%20Component _returnvalue_2))
        (SplineMesh|SetStartandEnd _output_get_2 (Spline|GetLocationatSplinePoint _spline_2 _index "Local") (Spline|GetLeaveTangentatSplinePoint _spline_2 _index "Local") (Spline|GetLocationatSplinePoint _spline (+ _index 1) "Local") (Spline|GetArriveTangentatSplinePoint _spline (+ _index 1) "Local") true :!class /Script/Engine.SplineMeshComponent)
        (SplineMesh|SetSplineUpDir (LocalVariables|GetLocal%20SMesh%20Component) (CallFunction|ComputeSplineMeshUpVector (Spline|GetLeaveTangentatSplinePoint _spline_2 _index "Local") (Spline|GetArriveTangentatSplinePoint _spline (+ _index 1) "Local")) true)
        (Rendering|Material|SetMaterial (LocalVariables|GetLocal%20SMesh%20Component) 0 (Variables|Default|GetDynamicMaterialInstance))))
    (:then_2
      (CallFunction|SetPlug false)
      (CallFunction|SetPlug true))))

(fn ComputeSplineMeshUpVector
  (params (TangentA :type Vector) (TangentB :type Vector))
  (Utilities|FlowControl|Sequence
    (:then_0
      (LocalVariables|SetTanA (Math|Vector|Normalize TangentA))
      (LocalVariables|SetTanB (Math|Vector|Normalize TangentB)))
    (:then_1
      (bind _output_get (LocalVariables|SetDot (Math|Vector|DotProduct (LocalVariables|GetTanA) (LocalVariables|GetTanB))))
      (if (or (> _output_get 0.99) (<= _output_get -0.99))
        (return (Math|Vector|MakeVector (.Y (Math|Vector|BreakVector (LocalVariables|GetTanA))) (.Z (Math|Vector|BreakVector (LocalVariables|GetTanA))) (.X (Math|Vector|BreakVector (LocalVariables|GetTanA)))))
        (else
          (return (Math|Vector|CrossProduct (LocalVariables|GetTanA) (LocalVariables|GetTanB))))))))

(fn SetPlug
  (params (End%20Plug :type Boolean))
  (bind _output_get (LocalVariables|SetLocal%20is%20End End%20Plug))
  (LocalVariables|SetLocal%20Plug%20Type (select _output_get (Variables|EndPlug|GetEnd%20Plug%20Type) (Variables|StartPlug|GetStart%20Plug%20Type)))
  (LocalVariables|SetLocal%20Type%20Offset (CallFunction|GetTypeOffset (LocalVariables|GetLocal%20Plug%20Type)))
  (LocalVariables|SetLocal%20Socket (select (LocalVariables|GetLocal%20is%20End) (Variables|EndPlug|GetEnd%20Socket) (Variables|StartPlug|GetStart%20Socket)))
  (LocalVariables|SetLocal%20Socket%20Place%20Number (select (LocalVariables|GetLocal%20is%20End) (Variables|EndPlug|GetEnd%20Socket%20Place%20Number) (Variables|StartPlug|GetStart%20Socket%20Place%20Number)))
  (LocalVariables|SetLocal%20is%20Plugged (select (LocalVariables|GetLocal%20is%20End) (Variables|EndPlug|GetEnd%20is%20Plugged) (Variables|StartPlug|GetStart%20is%20Plugged)))
  (LocalVariables|SetLocal%20Rotation (select (LocalVariables|GetLocal%20is%20End) (Variables|EndPlug|GetEnd%20Rotation) (Variables|StartPlug|GetStart%20Rotation)))
  (Variables|Default|SetLocal%20Flipped (select (LocalVariables|GetLocal%20is%20End) (Variables|EndPlug|GetEnd%20Flip) (Variables|StartPlug|GetStart%20Flip)))
  (if (not (Utilities|Enum|Equal(Enum) (LocalVariables|GetLocal%20Plug%20Type) "NewEnumerator3"))
    (bind _returnvalue (AddComponent|AddStaticMeshComponent false (Math|Transform|MakeTransform (.Location (Spline|GetLocationandTangentatSplinePoint (Variables|Default|GetSpline) (select (LocalVariables|GetLocal%20is%20End) (- (Spline|GetNumberOfSplinePoints (Variables|Default|GetSpline)) 1) 0) "Local")) (select (LocalVariables|GetLocal%20is%20Plugged) (Math|Rotator|CombineRotators (Math|Rotator|CombineRotators (.rotation (CallFunction|GetTypeOffset (LocalVariables|GetLocal%20Plug%20Type))) (.rotation (Utilities|GetSocket (LocalVariables|GetLocal%20Socket) (LocalVariables|GetLocal%20Socket%20Place%20Number) (Variables|Default|GetLocal%20Flipped)))) (Class|KismetMathLibrary|NegateRotator (Transformation|GetActorRotation))) (Math|Rotator|CombineRotators (Math|Rotator|MakeRotator (LocalVariables|GetLocal%20Rotation) 0.0 0.0) (select (LocalVariables|GetLocal%20is%20End) (Math|Rotator|CombineRotators "0.000000,180.000000,0.000000" (Math|Conversions|RotationFromXVector (.Tangent (Spline|GetLocationandTangentatSplinePoint (Variables|Default|GetSpline) (select (LocalVariables|GetLocal%20is%20End) (- (Spline|GetNumberOfSplinePoints (Variables|Default|GetSpline)) 1) 0) "Local")))) (Math|Conversions|RotationFromXVector (.Tangent (Spline|GetLocationandTangentatSplinePoint (Variables|Default|GetSpline) (select (LocalVariables|GetLocal%20is%20End) (- (Spline|GetNumberOfSplinePoints (Variables|Default|GetSpline)) 1) 0) "Local")))))) "1,1,1")))
    (bind _returnvalue_2 (Rendering|Material|CreateDynamicMaterialInstance _returnvalue 0 0 :!class /Script/Engine.PrimitiveComponent))
    (LocalVariables|SetDynamat _returnvalue_2)
    (Components|StaticMesh|SetStaticMesh _returnvalue (select (LocalVariables|GetLocal%20is%20Plugged) (Utilities|Select :Index (LocalVariables|GetLocal%20Plug%20Type) :NewEnumerator0 "/Game/BasicOffice/Meshes/Cable/SM_Plug_Flat_Plugged.SM_Plug_Flat_Plugged" :NewEnumerator1 "/Game/BasicOffice/Meshes/Cable/SM_Plug_Slim_Plugged.SM_Plug_Slim_Plugged" :NewEnumerator2 "/Game/BasicOffice/Meshes/Cable/SM_Plug_USB_Plugged.SM_Plug_USB_Plugged" :NewEnumerator3 0) (Utilities|Select :Index (LocalVariables|GetLocal%20Plug%20Type) :NewEnumerator0 "/Game/BasicOffice/Meshes/Cable/SM_Plug_Flat.SM_Plug_Flat" :NewEnumerator1 "/Game/BasicOffice/Meshes/Cable/SM_Plug_Slim.SM_Plug_Slim" :NewEnumerator2 "/Game/BasicOffice/Meshes/Cable/SM_Plug_USB.SM_Plug_USB" :NewEnumerator3 0)))
    (Rendering|Material|SetVectorParameterValue (LocalVariables|GetDynamat) "TintColor" (Variables|Cable|GetColor) :!class /Script/Engine.MaterialInstanceDynamic)))

(fn PlugtoSocket
  (params (is%20End :type Boolean))
  (bind _output_get (LocalVariables|SetLocal%20is%20End is%20End))
  (LocalVariables|SetLocal%20Socket (select _output_get (Variables|EndPlug|GetEnd%20Socket) (Variables|StartPlug|GetStart%20Socket)))
  (LocalVariables|SetLocal%20Flipped (select (LocalVariables|GetLocal%20is%20End) (Variables|EndPlug|GetEnd%20Flip) (Variables|StartPlug|GetStart%20Flip)))
  (LocalVariables|SetLocal%20Plug%20Type (select (LocalVariables|GetLocal%20is%20End) (Variables|EndPlug|GetEnd%20Plug%20Type) (Variables|StartPlug|GetStart%20Plug%20Type)))
  (LocalVariables|SetLocal%20Socket%20Place%20Number (select (LocalVariables|GetLocal%20is%20End) (Variables|EndPlug|GetEnd%20Socket%20Place%20Number) (Variables|StartPlug|GetStart%20Socket%20Place%20Number)))
  (LocalVariables|SetLocal%20Type%20Offset (CallFunction|GetTypeOffset (LocalVariables|GetLocal%20Plug%20Type)))
  (Utilities|IsValid (LocalVariables|GetLocal%20Socket)
    (:Is%20Valid
      (Utilities|FlowControl|Sequence
        (:then_0
          (if (LocalVariables|GetLocal%20is%20End)
            (Variables|EndPlug|SetEnd%20is%20Plugged true)
            (else
              (Variables|StartPlug|SetStart%20is%20Plugged true))))
        (:then_1
          (Spline|SetLocationatSplinePoint (Variables|Default|GetSpline) (select (LocalVariables|GetLocal%20is%20End) (- (Spline|GetNumberOfSplinePoints (Variables|Default|GetSpline)) 1) 0) (.location (Math|Transform|ComposeTransforms (LocalVariables|GetLocal%20Type%20Offset) (Utilities|GetSocket (LocalVariables|GetLocal%20Socket) (LocalVariables|GetLocal%20Socket%20Place%20Number) (LocalVariables|GetLocal%20Flipped)))) "World" true)
          (Spline|SetTangentatSplinePoint (Variables|Default|GetSpline) (select (LocalVariables|GetLocal%20is%20End) (- (Spline|GetNumberOfSplinePoints (Variables|Default|GetSpline)) 1) 0) (* (Math|Vector|GetForwardVector (.rotation (Math|Transform|ComposeTransforms (LocalVariables|GetLocal%20Type%20Offset) (Utilities|GetSocket (LocalVariables|GetLocal%20Socket) (LocalVariables|GetLocal%20Socket%20Place%20Number) (LocalVariables|GetLocal%20Flipped))))) (select (LocalVariables|GetLocal%20is%20End) (Variables|EndPlug|GetEnd%20Tangent) (Variables|StartPlug|GetStart%20Tangent))) "World" true))))
    (:Is%20Not%20Valid
      (if (LocalVariables|GetLocal%20is%20End)
        (Variables|EndPlug|SetEnd%20is%20Plugged false)
        (else
          (Variables|StartPlug|SetStart%20is%20Plugged false))))))

(fn GetTypeOffset
  (params (Index :type E_OfficeCableType%20Enum))
  (return (Utilities|Select :Index Index :NewEnumerator0 (Math|Transform|MakeTransform "0,-4.800000,3.000000" "0.000000,-90.000000,0.000000" "1,1,1") :NewEnumerator1 (Math|Transform|MakeTransform "0, 0,5.000000" "90.000000,90.000000, 0" "1,1,1") :NewEnumerator2 (Math|Transform|MakeTransform "0, 0,3.200000" "90.000000,0.000000,90.000000" "1,1,1") :NewEnumerator3 (Math|Transform|MakeTransform "0, 0, 0" "90.000000,0.000000, 0" "1,1,1"))))