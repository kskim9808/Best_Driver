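; Cork board prop that scatters random pins and pinned papers across its surface in the construction script.
; Pins and papers use instanced mesh components with inverse actor scale, so the board can scale while instances keep their size.
; PositionSeed stream drives placement and rotation, reseeded when RandomPositions is on; PaperSeed at or below 0.01 sets the paper material's Phase.
; Each paper adds a pin to the Pins component, created only when NumberOfRandomPins exceeds zero.
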(fn ConstructionScript
  (if (Variables|Default|GetRandom%20Positions)
    (Math|Random|SetRandomStreamSeed (Variables|Default|GetPosition%20Seed) (Math|Random|RandomInteger 999)))
  (CallFunction|GeneratePinsandPaper))

(fn GeneratePinsandPaper
  (bind _returnvalue (Transformation|GetActorScale3D))
  (bind _returnvalue_2 (Transformation|GetActorScale3D))
  (bind _returnvalue_3 (/ "1.000000,1.000000,1.000000" _returnvalue))
  (bind _returnvalue_4 (/ (.z _returnvalue_2) 5.0))
  (Utilities|FlowControl|Sequence
    (:then_0
      (if (> (Variables|Default|GetNumber%20of%20Random%20Pins) 0)
        (bind _returnvalue_5 (AddComponent|AddInstancedStaticMeshComponent false (Math|Transform|MakeTransform "0, 0, 0" "0, 0, 0" _returnvalue_3)))
        (Variables|Default|SetPins _returnvalue_5)
        (for _index (range 0 (- (Variables|Default|GetNumber%20of%20Random%20Pins) 1))
          (Components|InstancedStaticMesh|AddInstance (Variables|Default|GetPins) (Math|Transform|MakeTransform (* (Math|Vector|MakeVector (Math|Random|RandomFloatinRangefromStream -27.0 27.0 (Variables|Default|GetPosition%20Seed)) (Math|Random|RandomFloatinRangefromStream -17.0 17.0 (Variables|Default|GetPosition%20Seed)) 0.0) (Transformation|GetActorScale3D)) (Math|Rotator|MakeRotator (Math|Random|RandomFloatinRangefromStream -3e+01 3e+01 (Variables|Default|GetPosition%20Seed)) 0.0 (Math|Random|RandomFloatinRangefromStream -3e+01 3e+01 (Variables|Default|GetPosition%20Seed))) "1.000000,1.000000,1.000000")))))
    (:then_1
      (if (> (Variables|Default|GetNumber%20of%20Papers) 0)
        (bind _returnvalue_6 (AddComponent|AddInstancedStaticMeshComponent false (Math|Transform|MakeTransform "0, 0, 0" "0, 0, 0" _returnvalue_3)))
        (bind _output_get (Variables|Default|SetPapers _returnvalue_6))
        (if (<= (Variables|Default|GetPaper%20Seed) 0.01)
          (bind _returnvalue_7 (Rendering|Material|CreateDynamicMaterialInstance _output_get 0 0 :!class /Script/Engine.PrimitiveComponent))
          (Rendering|Material|SetScalarParameterValue _returnvalue_7 "Phase" (/ (Variables|Default|GetPaper%20Seed) 1e+02) :!class /Script/Engine.MaterialInstanceDynamic))
        (for _index_2 (range 0 (- (Variables|Default|GetNumber%20of%20Papers) 1))
          (bind _output_get_2 (LocalVariables|SetLocal%20PaperPos (+ (* (Math|Vector|MakeVector (Math|Random|RandomFloatinRangefromStream -17.0 17.0 (Variables|Default|GetPosition%20Seed)) (Math|Random|RandomFloatinRangefromStream -1e+01 1e+01 (Variables|Default|GetPosition%20Seed)) (Math|Random|RandomFloatinRangefromStream _returnvalue_4 (+ _returnvalue_4 0.1) (Variables|Default|GetPosition%20Seed))) (Transformation|GetActorScale3D)) "0, 0,1.200000")))
          (Components|InstancedStaticMesh|AddInstance (Variables|Default|GetPapers) (Math|Transform|MakeTransform _output_get_2 (Math|Rotator|MakeRotator 0.0 0.0 (Math|Random|RandomFloatinRangefromStream -25.0 25.0 (Variables|Default|GetPosition%20Seed))) "1.000000,1.000000,1.000000"))
          (Components|InstancedStaticMesh|AddInstance (Variables|Default|GetPins) (Math|Transform|MakeTransform (+ (LocalVariables|GetLocal%20PaperPos) (Math|Vector|MakeVector 0.0 (Math|Random|RandomFloatinRangefromStream 3.0 6.0 (Variables|Default|GetPosition%20Seed)) 0.0)) (Math|Rotator|MakeRotator (Math|Random|RandomFloatinRangefromStream 0.0 4e+01 (Variables|Default|GetPosition%20Seed)) 0.0 (Math|Random|RandomFloatinRangefromStream -15.0 15.0 (Variables|Default|GetPosition%20Seed))) "1.000000,1.000000,1.000000")))))))