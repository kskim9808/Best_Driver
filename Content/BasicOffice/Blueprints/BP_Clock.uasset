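; BP_Clock is a clock prop whose displayed time is set per instance through Hours and Minutes values.
; The construction script optionally adds an audio component when WithSound is enabled.
; It then creates a dynamic material instance on ClockMesh and passes both time values to it as scalar parameters, leaving the display to the material.
; The event graph holds only disabled placeholder events, so the Blueprint runs no runtime update logic.
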(event EventBeginPlay)

(event Collision|EventActorBeginOverlap
  (params (OtherActor :type Actor%20Object%20Reference)))

(event EventTick
  (params (DeltaSeconds :type Float%20%28single-precision%29)))

(fn ConstructionScript
  (Utilities|FlowControl|Sequence
    (:then_0
      (if (Variables|Default|GetWith%20Sound)
        (AddComponent|AddAudioComponent false)))
    (:then_1
      (bind _returnvalue (Rendering|Material|CreateDynamicMaterialInstance (Variables|Default|GetClockMesh) 0 0 :!class /Script/Engine.PrimitiveComponent))
      (bind _output_get (Variables|Default|SetDynamat _returnvalue))
      (Rendering|Material|SetScalarParameterValue _output_get "Hours" (Variables|Default|GetHours) :!class /Script/Engine.MaterialInstanceDynamic)
      (Rendering|Material|SetScalarParameterValue (Variables|Default|GetDynamat) "Minutes" (Variables|Default|GetMinutes) :!class /Script/Engine.MaterialInstanceDynamic))))