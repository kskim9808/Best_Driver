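; Modular office wall-with-window actor, configured entirely in its construction script.
; GlowFog and TranslucentGlowFog pick a hidden, glow or simple glow material for the window frame's second slot, as a dynamic instance driven by Distance.
; Open swaps the frame mesh and the socket for optional blinds, added as a runtime-created component.
; Dynamic blinds use their own material instance to control closing and roll-up.
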(event EventBeginPlay)

(event Collision|EventActorBeginOverlap
  (params (OtherActor :type Actor%20Object%20Reference)))

(event EventTick
  (params (DeltaSeconds :type Float%20%28single-precision%29)))

(fn ConstructionScript
  (bind _returnvalue (Rendering|Material|CreateDynamicMaterialInstance (Variables|Default|GetSM_BldWndFrm_01_) 1 (Utilities|Select :Index (Math|Integer|SelectInt (Math|Integer|SelectInt 1 2 (Variables|GlowFog|GetTranslucentGlowFog)) 0 (Variables|GlowFog|GetGlowFog)) :Option%200 "/Game/BasicOffice/Materials/Window/M_HideMat.M_HideMat" :Option%201 "/Game/BasicOffice/Materials/Window/M_GlowOutside.M_GlowOutside" :Option%202 "/Game/BasicOffice/Materials/Window/M_GlowOutsideSimple.M_GlowOutsideSimple") :!class /Script/Engine.PrimitiveComponent))
  (Rendering|Material|SetScalarParameterValue _returnvalue "Distance" (Variables|GlowFog|GetDistance) :!class /Script/Engine.MaterialInstanceDynamic)
  (Components|StaticMesh|SetStaticMesh (Variables|Default|GetSM_BldWndFrm_01_) (select (Variables|Window|GetOpen) "/Game/BasicOffice/Meshes/Building/SM_BldWndFrm_01-Open_.SM_BldWndFrm_01-Open_" "/Game/BasicOffice/Meshes/Building/SM_BldWndFrm_01_.SM_BldWndFrm_01_"))
  (if (Variables|Blinds|GetBlinds)
    (bind _returnvalue_2 (AddComponent|AddStaticMeshComponent true))
    (bind _output_get (Variables|Default|SetBlinds_Component _returnvalue_2))
    (Transformation|AttachComponentToComponent _output_get (select (Variables|Window|GetOpen) (Variables|Default|GetBlinds_SocketOpen) (Variables|Default|GetBlinds_Socket)) "None" "SnapToTarget" "SnapToTarget" "SnapToTarget" true)
    (Components|StaticMesh|SetStaticMesh (Variables|Default|GetBlinds_Component) (select (Variables|Blinds|GetDynamic%20Blinds) "/Game/BasicOffice/Meshes/SM_BlindsDynamic.SM_BlindsDynamic" "/Game/BasicOffice/Meshes/SM_Blinds.SM_Blinds"))
    (if (Variables|Blinds|GetDynamic%20Blinds)
      (bind _returnvalue_3 (Rendering|Material|CreateDynamicMaterialInstance (Variables|Default|GetBlinds_Component) 0 0 :!class /Script/Engine.PrimitiveComponent))
      (Rendering|Material|SetScalarParameterValue _returnvalue_3 "Closed" (Variables|Blinds|GetClosed) :!class /Script/Engine.MaterialInstanceDynamic)
      (Rendering|Material|SetScalarParameterValue _returnvalue_3 "Role Up" (Variables|Blinds|GetRole%20Up) :!class /Script/Engine.MaterialInstanceDynamic))))