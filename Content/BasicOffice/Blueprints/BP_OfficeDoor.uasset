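; BP_OfficeDoor is a configurable office door prop, set up entirely in its construction script with no active runtime logic.
; The construction script picks one of five handle meshes from KnopType, then applies frame, door and knob colors through dynamic material instances.
; It also poses the door by mapping DoorState as a percentage onto the hinge's yaw, from closed to swung wide open.
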(event EventBeginPlay)

(event Collision|EventActorBeginOverlap
  (params (OtherActor :type Actor%20Object%20Reference)))

(event EventTick
  (params (DeltaSeconds :type Float%20%28single-precision%29)))

(fn ConstructionScript
  (Components|StaticMesh|SetStaticMesh (Variables|Default|GetSM_klinke02) (Utilities|Select :Index (Variables|Default|GetKnopType) :Option%200 "/Game/BasicOffice/Meshes/Door/SM_Handle01.SM_Handle01" :Option%201 "/Game/BasicOffice/Meshes/Door/SM_Handle02.SM_Handle02" :Option%202 "/Game/BasicOffice/Meshes/Door/SM_Handle03.SM_Handle03" :Option%203 "/Game/BasicOffice/Meshes/Door/SM_Handle04.SM_Handle04" :Option%204 "/Game/BasicOffice/Meshes/Door/SM_Handle05.SM_Handle05"))
  (CallFunction|SetDynamicMaterials)
  (CallFunction|UpdateDoorState))

(fn UpdateDoorState
  (Transformation|SetRelativeRotation (Variables|Default|GetHinge) (Math|Rotator|MakeRotator 0.0 0.0 (Math|Float|Lerp 0.0 165.0 (/ (Variables|Default|GetDoorState) 1e+02))) false false))

(fn SetDynamicMaterials
  (bind _returnvalue (Rendering|Material|CreateDynamicMaterialInstance (Variables|Default|GetFrame) 0 0 :!class /Script/Engine.PrimitiveComponent))
  (Rendering|Material|SetVectorParameterValue _returnvalue "Color" (Variables|Default|GetFrameColor) :!class /Script/Engine.MaterialInstanceDynamic)
  (bind _returnvalue_2 (Rendering|Material|CreateDynamicMaterialInstance (Variables|Default|GetSM_Door) 0 0 :!class /Script/Engine.PrimitiveComponent))
  (Rendering|Material|SetVectorParameterValue _returnvalue_2 "Color" (Variables|Default|GetDoorColor) :!class /Script/Engine.MaterialInstanceDynamic)
  (bind _returnvalue_3 (Rendering|Material|CreateDynamicMaterialInstance (Variables|Default|GetSM_Door) 1 0 :!class /Script/Engine.PrimitiveComponent))
  (Rendering|Material|SetVectorParameterValue _returnvalue_3 "TintColor" (Variables|Default|GetDoorKnopColor) :!class /Script/Engine.MaterialInstanceDynamic)
  (bind _returnvalue_4 (Rendering|Material|CreateDynamicMaterialInstance (Variables|Default|GetSM_klinke02) 0 0 :!class /Script/Engine.PrimitiveComponent))
  (Rendering|Material|SetVectorParameterValue _returnvalue_4 "TintColor" (Variables|Default|GetDoorKnopColor) :!class /Script/Engine.MaterialInstanceDynamic))