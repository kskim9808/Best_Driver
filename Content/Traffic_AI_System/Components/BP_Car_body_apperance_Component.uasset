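; Traffic AI vehicle component that sets up a car's body color and lighting, using the owner's mesh root component.
; Setup spawns shadowless front and rear spot lights with light functions, positioned from mesh bounds.
; It creates dynamic materials on the "Lights" and "Body" slots, picking a random color or the array's last.
; Events toggle indicators, hazards, headlights, brake and reverse lights through material parameters, also adjusting spot intensity for headlights and braking.
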(event Custom|Set%20up%20car%20body
  (params (Owner :type Actor%20Object%20Reference) (Car%20Body :type Mesh%20Component%20Object%20Reference))
  (bind _car_colors (Variables|Color|GetCar%20Colors))
  (bind _returnvalue (Utilities|Array|LastIndex _car_colors))
  (Utilities|FlowControl|Sequence
    (:then_0
      (Variables|System|SetOwner Owner)
      (Variables|Default|SetCar%20Body%20mesh Car%20Body))
    (:then_1
      ;[1 0.7401 0.4135] Add head light (one spot light with light function)
      (bind _returnvalue_2 (Game|AddComponentbyClass (Variables|System|GetOwner) "/Script/Engine.SpotLightComponent" false (Math|Transform|MakeTransform (Math|Vector|MakeVector (+ (.X (Math|Vector|BreakVector (select (.bSuccess (Utilities|Casting|CastToSkeletalMeshComponent (Variables|Default|GetCar%20Body%20mesh))) (.origin (Class|SkeletalMesh|GetImportedBounds (Variables|/Script/Engine.SkinnedMeshComponent|GetSkeletalMesh (.AsSkeletal%20Mesh%20Component (Utilities|Casting|CastToSkeletalMeshComponent (Variables|Default|GetCar%20Body%20mesh)))))) (.Origin (Collision|GetComponentBounds (Variables|Default|GetCar%20Body%20mesh)))))) (select (.bSuccess (Utilities|Casting|CastToSkeletalMeshComponent (Variables|Default|GetCar%20Body%20mesh))) (.x (.boxextent (Class|SkeletalMesh|GetImportedBounds (Variables|/Script/Engine.SkinnedMeshComponent|GetSkeletalMesh (.AsSkeletal%20Mesh%20Component (Utilities|Casting|CastToSkeletalMeshComponent (Variables|Default|GetCar%20Body%20mesh))))))) (.x (.BoxExtent (Collision|GetComponentBounds (Variables|Default|GetCar%20Body%20mesh)))))) 0.0 (Variables|Lights|GetFront%20light%20Z%20offset)) "-10.000000, 0,0.000000" "1,1,1")))
      (Rendering|Components|Light|SetCastShadows _returnvalue_2 false)
      (Rendering|Components|Light|SetIntensity _returnvalue_2 (Variables|Lights|GetFront%20Light%20intensity))
      (Rendering|Components|Light|SetLightColor _returnvalue_2 (Variables|Lights|GetFront%20light%20color) true)
      (Rendering|Lighting|SetAttenuationRadius _returnvalue_2 (Variables|Lights|GetFront%20light%20radius))
      (Rendering|Lighting|SetOuterConeAngle _returnvalue_2 (Variables|Lights|GetFront%20light%20Outer%20Cone%20Angle))
      (Rendering|Components|Light|SetLightFunctionMaterial _returnvalue_2 (Variables|Lights|GetFront%20light%20material%20function))
      (Variables|Default|SetFront%20light _returnvalue_2))
    (:then_2
      ;[1 0.1668 0.06708] Add tail light (one spot light with light function)
      (bind _returnvalue_3 (Game|AddComponentbyClass (Variables|System|GetOwner) "/Script/Engine.SpotLightComponent" false (Math|Transform|MakeTransform (Math|Vector|MakeVector (* (- (* (select (.bSuccess (Utilities|Casting|CastToSkeletalMeshComponent (Variables|Default|GetCar%20Body%20mesh))) (.x (.boxextent (Class|SkeletalMesh|GetImportedBounds (Variables|/Script/Engine.SkinnedMeshComponent|GetSkeletalMesh (.AsSkeletal%20Mesh%20Component (Utilities|Casting|CastToSkeletalMeshComponent (Variables|Default|GetCar%20Body%20mesh))))))) (.x (.BoxExtent (Collision|GetComponentBounds (Variables|Default|GetCar%20Body%20mesh))))) 1.1) (.X (Math|Vector|BreakVector (select (.bSuccess (Utilities|Casting|CastToSkeletalMeshComponent (Variables|Default|GetCar%20Body%20mesh))) (.origin (Class|SkeletalMesh|GetImportedBounds (Variables|/Script/Engine.SkinnedMeshComponent|GetSkeletalMesh (.AsSkeletal%20Mesh%20Component (Utilities|Casting|CastToSkeletalMeshComponent (Variables|Default|GetCar%20Body%20mesh)))))) (.Origin (Collision|GetComponentBounds (Variables|Default|GetCar%20Body%20mesh))))))) -1.0) 0.0 (Variables|Lights|GetRear%20light%20Z%20offset)) "0,180.000000, 0" "1,1,1")))
      (Rendering|Components|Light|SetCastShadows _returnvalue_3 false)
      (Rendering|Components|Light|SetIntensity _returnvalue_3 (Variables|Lights|GetRear%20light%20intencity))
      (Rendering|Components|Light|SetLightColor _returnvalue_3 (Variables|Lights|GetRear%20light%20color) true)
      (Rendering|Lighting|SetAttenuationRadius _returnvalue_3 (Variables|Lights|GetRear%20light%20radius))
      (Rendering|Lighting|SetOuterConeAngle _returnvalue_3 (Variables|Lights|GetRear%20light%20angle))
      (Rendering|Components|Light|SetLightFunctionMaterial _returnvalue_3 (Variables|Lights|GetRear%20light%20material%20function))
      (Variables|Default|SetRear%20Light _returnvalue_3))
    (:then_3
      ;[0.08653 0.329 1] Create material instance for light on mesh and save it as a variable
      (if (not (== (Utilities|Array|FindItem (Class|MeshComponent|GetMaterialSlotNames (Variables|Default|GetCar%20Body%20mesh)) "Lights") -1))
        (bind _returnvalue_4 (Rendering|Material|CreateDynamicMaterialInstance (Variables|Default|GetCar%20Body%20mesh) (Utilities|Array|FindItem (Class|MeshComponent|GetMaterialSlotNames (Variables|Default|GetCar%20Body%20mesh)) "Lights") (Rendering|Material|GetMaterial (Variables|Default|GetCar%20Body%20mesh) (Utilities|Array|FindItem (Class|MeshComponent|GetMaterialSlotNames (Variables|Default|GetCar%20Body%20mesh)) "Lights")) "None" :!class /Script/Engine.PrimitiveComponent))
        (Variables|System|SetLights%20material%20instance _returnvalue_4)
        (Rendering|Material|SetVectorParameterValue _returnvalue_4 "Front Lights Color" (Variables|Lights|GetFront%20light%20color) :!class /Script/Engine.MaterialInstanceDynamic)
        (Rendering|Material|SetScalarParameterValue _returnvalue_4 "Random per instance" (Math|Random|RandomFloatinRange 0.0 1.0) :!class /Script/Engine.MaterialInstanceDynamic)))
    (:then_4
      ;[0.9019 0.377 1] Set car color
      (if (not (== (Utilities|Array|FindItem (Class|MeshComponent|GetMaterialSlotNames (Variables|Default|GetCar%20Body%20mesh)) "Body") -1))
        (bind _returnvalue_5 (Rendering|Material|CreateDynamicMaterialInstance (Variables|Default|GetCar%20Body%20mesh) (Utilities|Array|FindItem (Class|MeshComponent|GetMaterialSlotNames (Variables|Default|GetCar%20Body%20mesh)) "Body") (Rendering|Material|GetMaterial (Variables|Default|GetCar%20Body%20mesh) (Utilities|Array|FindItem (Class|MeshComponent|GetMaterialSlotNames (Variables|Default|GetCar%20Body%20mesh)) "Body")) "None" :!class /Script/Engine.PrimitiveComponent))
        (bind _output_get (Variables|System|SetBody%20Material%20Instance _returnvalue_5))
        (Rendering|Material|SetVectorParameterValue _output_get "Color" (Utilities|Array|Get(acopy) _car_colors (select (Variables|Color|GetSpecific%20color?) _returnvalue (Math|Random|RandomIntegerinRange 0 _returnvalue))) :!class /Script/Engine.MaterialInstanceDynamic)))))

(event Custom|Enable%20indicator
  (params (Indicator%20type :type Enum_TurnType%20Enum :default "NewEnumerator0") (Hazard? :type Boolean) (Temporary? :type Boolean))
  ;[1 0.4466 0.183] Toggle indicator
  (Variables|Default|SetTemporary%20indicator Temporary?)
  (Variables|System|SetIndicator%20state Indicator%20type)
  (Variables|Lights|SetHazard? Hazard?) ; Added in 1.1 update
  (Rendering|Material|SetScalarParameterValue (Variables|System|GetLights%20material%20instance) "Right indicator on" (select (Variables|Lights|GetHazard?) 1.0 (Utilities|Select :Index Indicator%20type :NewEnumerator0 0.0 :NewEnumerator1 1.0 :NewEnumerator2 0.0)) :!class /Script/Engine.MaterialInstanceDynamic)
  (Rendering|Material|SetScalarParameterValue (Variables|System|GetLights%20material%20instance) "Left indicator on" (select (Variables|Lights|GetHazard?) 1.0 (Utilities|Select :Index Indicator%20type :NewEnumerator0 0.0 :NewEnumerator1 0.0 :NewEnumerator2 1.0)) :!class /Script/Engine.MaterialInstanceDynamic))

(event Custom|Enable%20headlights
  (params (Enable? :type Boolean))
  ;[0.4463 1 0.9602] Toggle headlights
  (Variables|System|SetHeadlights%20on? Enable?)
  (Rendering|Material|SetScalarParameterValue (Variables|System|GetLights%20material%20instance) "Front Lights on" (Math|Conversions|ToFloat(Boolean) Enable?) :!class /Script/Engine.MaterialInstanceDynamic)
  (Rendering|Components|Light|SetIntensity (Variables|Default|GetFront%20light) (select (Variables|System|GetHeadlights%20on?) (Variables|Lights|GetFront%20Light%20intensity) 0.0))
  (Rendering|Components|Light|SetIntensity (Variables|Default|GetRear%20Light) (select (Variables|System|GetHeadlights%20on?) (Variables|Lights|GetRear%20light%20intencity) 0.0)))

(event Custom|Brake%20light
  (params (Enable? :type Boolean))
  ;[0.3073 1 0.3073] Toggle Brake lights
  (Variables|System|SetBrake%20light%20enabled? Enable?)
  (Rendering|Material|SetScalarParameterValue (Variables|System|GetLights%20material%20instance) "Brake light on" (Math|Conversions|ToFloat(Boolean) Enable?) :!class /Script/Engine.MaterialInstanceDynamic)
  (Rendering|Components|Light|SetIntensity (Variables|Default|GetRear%20Light) (select Enable? (* (Variables|Lights|GetRear%20light%20intencity) 3.0) (select (Variables|System|GetHeadlights%20on?) (Variables|Lights|GetRear%20light%20intencity) 0.0))))

(event Custom|Enable%20Reverse%20Light
  (params (Enabled? :type Boolean))
  ;[1 1 1] Reverse Light
  (Rendering|Material|SetScalarParameterValue (Variables|System|GetLights%20material%20instance) "Reverse light on" (Math|Conversions|ToFloat(Boolean) Enabled?) :!class /Script/Engine.MaterialInstanceDynamic))

(event EventBeginPlay
  (bind _returnvalue (Components|GetOwner))
  (bind _asmesh_component (Utilities|Casting|CastToMeshComponent (Variables|/Script/Engine.Actor|GetRootComponent _returnvalue))
    (:then
      (CallFunction|SetUpCarBody _returnvalue _asmesh_component))
    (:CastFailed
      (Development|PrintString "Traffic AI System error: Root component of your vehicle is not a mesh" true true "(R=1.000000,G=0.000000,B=0.007126,A=1.000000)" 5.0))))