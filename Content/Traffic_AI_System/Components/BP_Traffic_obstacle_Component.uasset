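; Actor component for the traffic AI system that tracks its owner's position along the current road and manages actor registration on that road.
; A looping timer, created paused on BeginPlay, updates DistanceOnRoad by interpolating between spline point distances on the road's SecondSpline.
; Owners not yet on the spline get a negative straight-line distance to its first point.
; Add and remove events update the road's unsorted actor array and trigger re-sorting.
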(event Custom|Set%20Distance%20on%20road
  (bind _self self)
  (bind _current_road (Variables|Default|GetCurrent%20road))
  (bind _returnvalue (Components|GetOwner _self))
  (bind _second_spline (Variables|/Game/Traffic_AI_System/Blueprints/BP_Traffic_path_50_Parent.BP_Traffic_path_50_Parent_C|GetSecond%20spline _current_road))
  (bind _returnvalue_2 (Transformation|GetActorLocation _returnvalue))
  (bind _returnvalue_3 (Class|SplineComponent|FindInputKeyClosesttoWorldLocation _second_spline _returnvalue_2))
  (bind _returnvalue_4 (Math|Float|Truncate _returnvalue_3))
  (bind _returnvalue_5 (+ _returnvalue_3 1.0))
  (bind _returnvalue_6 (Math|Float|Truncate _returnvalue_5))
  (bind _returnvalue_7 (Spline|GetDistanceAlongSplineatSplinePoint _second_spline _returnvalue_4))
  (bind _returnvalue_8 (Math|Conversions|ToFloat(Integer) _returnvalue_4))
  (bind _returnvalue_9 (Spline|GetDistanceAlongSplineatSplinePoint _second_spline _returnvalue_6))
  (bind _returnvalue_10 (- _returnvalue_3 _returnvalue_8))
  (bind _returnvalue_11 (- _returnvalue_9 _returnvalue_7))
  (bind _returnvalue_12 (* _returnvalue_11 _returnvalue_10))
  (bind _returnvalue_13 (+ _returnvalue_7 _returnvalue_12))
  (Utilities|IsValid (Variables|Default|GetCurrent%20road)
    (:Is%20Valid
      (if (<= _returnvalue_13 0.0)
        ;[1 0.6169 0.2965] Set negative Distance on Road in case that car did not arrived to the spline yet
        (Variables|Default|SetDistance%20on%20road (* (Math|Vector|Distance(Vector) (Transformation|GetActorLocation (Components|GetOwner self)) (Spline|GetLocationatSplinePoint (Variables|/Game/Traffic_AI_System/Blueprints/BP_Traffic_path_50_Parent.BP_Traffic_path_50_Parent_C|GetSecond%20spline (Variables|Default|GetCurrent%20road)) 0 "World")) -1.0))
        (else
          ;[0.4463 1 0.9602] Calculate distance on spline
          (Variables|Default|SetDistance%20on%20road _returnvalue_13))))))

(event Custom|Remove%20Actor%20From%20Road
  (params (Actor :type Actor%20Object%20Reference))
  (bind _current_road (Variables|Default|GetCurrent%20road))
  ;[1 0.7097 0.2625] Remove actor from the Road Array
  (Utilities|IsValid _current_road
    (:Is%20Valid
      (Utilities|Array|RemoveItem (Variables|/Game/Traffic_AI_System/Blueprints/BP_Traffic_path_50_Parent.BP_Traffic_path_50_Parent_C|GetActors%20unsorted _current_road) Actor)
      (Default|SortObjectsOrderArray _current_road))))

(event Custom|Add%20Actor%20To%20Road
  (params (Actor :type Actor%20Object%20Reference))
  (bind _current_road (Variables|Default|GetCurrent%20road))
  ;[0.2577 1 0.2174] Add actor to the Road Array
  (Utilities|IsValid _current_road
    (:Is%20Valid
      (Utilities|Array|AddUnique (Variables|/Game/Traffic_AI_System/Blueprints/BP_Traffic_path_50_Parent.BP_Traffic_path_50_Parent_C|GetActors%20unsorted _current_road) Actor)
      (Default|SortObjectsOrderArray _current_road))))

(event EventBeginPlay
  (bind _returnvalue (Utilities|Time|SetTimerbyEvent (delegate Custom|Set%20Distance%20on%20road) (Variables|Default|GetCalculate%20distance%20frequency) true))
  (bind _output_get (Variables|Default|SetCalculate%20distance%20timer _returnvalue))
  (Utilities|Time|PauseTimerbyHandle _output_get))