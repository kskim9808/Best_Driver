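; Preview pawn for the Traffic AI System that shows the preview UI and provides debug hotkeys.
; Keys advance the time of day with 24-hour wrap and raise or lower the main road's AI car limit.
; Enter finds the nearest physics-simulating traffic car, unpossesses its AI controller and possesses it as the player.
; It then adds a lagged spring-arm camera at runtime and switches the car to Drive mode.
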(event EventBeginPlay
  (bind _returnvalue (UserInterface|CreateWidget "/Game/Traffic_AI_System/Preview/Preview_blueprints/UI_Traffic_AI_Preview.UI_Traffic_AI_Preview_C"))
  (UserInterface|Viewport|AddtoViewport _returnvalue 0))

(event Input|KeyboardEvents|Enter
  (params (Key :type Key%20Structure :default "None"))
  (:Pressed
    (Variables|Default|SetDistance%20to%20nearest%20car 1e+10)
    ;[1 0.4664 0.923] Find the nearest car that simulates physics.
    (bind _outactors (Actor|GetAllActorsOfClass "/Game/Traffic_AI_System/Cars/BP_Traffic_car_parent.BP_Traffic_car_parent_C"))
    (for _array_element _outactors
      (if (Physics|IsSimulatingPhysics (Variables|/Script/PhysXVehicles.WheeledVehicle|GetMesh _array_element) "None")
        (if (< (Transformation|GetDistanceTo _array_element self) (Variables|Default|GetDistance%20to%20nearest%20car))
          (Variables|Default|SetDistance%20to%20nearest%20car (Transformation|GetDistanceTo _array_element self))
          (Variables|Default|SetClosest%20car _array_element))))
    ;[0.3844 1 0.7542] Possess the vehcle
    (bind _aspawn (Utilities|Casting|CastToPawn (Variables|Default|GetClosest%20car)))
    (Utilities|IsValid (AI|GetAIController _aspawn)
      (:Is%20Valid
        (Variables|Default|SetUnpossesed%20AI (AI|GetAIController _aspawn))
        (Pawn|UnPossess (AI|GetAIController _aspawn)))
      (:Is%20Not%20Valid
        _))
    (Pawn|Possess (Game|GetPlayerController 0) _aspawn)
    ;[1 0.7097 0.2625] Add Spring Arm and Camera components
    (bind _returnvalue (Game|AddComponentbyClass (Variables|Default|GetClosest%20car) "/Script/Engine.SpringArmComponent" false (Math|Transform|MakeTransform "0,0.000000,150.000000" "-15.000000, 0, 0" "1,1,1")))
    (Variables|/Script/Engine.SpringArmComponent|SetTargetArmLength _returnvalue 6e+02)
    (Variables|/Script/Engine.SpringArmComponent|SetbEnableCameraRotationLag _returnvalue true)
    (Variables|/Script/Engine.SpringArmComponent|SetCameraRotationLagSpeed _returnvalue 3.0)
    (bind _returnvalue_2 (Game|AddComponentbyClass (Variables|Default|GetClosest%20car) "/Script/Engine.CameraComponent" false))
    (Transformation|AttachComponentToComponent _returnvalue_2 _returnvalue "None" "SnapToTarget" "SnapToTarget" "SnapToTarget" true)
    ;[1 0.269 0.6684] Set car mode to "Drive", so that the player can controll it.
    (Default|SetCarModeEvent (Actor|GetComponentbyClass (Variables|Default|GetClosest%20car) "/Game/Traffic_AI_System/Components/BP_Traffic_Car_Component.BP_Traffic_Car_Component_C") "NewEnumerator2")))

(event Input|KeyboardEvents|Add
  (params (Key :type Key%20Structure :default "None"))
  ;[1 0.9353 0.4875] Inputs
  (:Pressed
    (bind _returnvalue (Actor|GetActorOfClass "/Game/Traffic_AI_System/Blueprints/BP_Traffic_path_50_Parent.BP_Traffic_path_50_Parent_C"))
    (Variables|/Game/Traffic_AI_System/Blueprints/BP_Traffic_path_50_Parent.BP_Traffic_path_50_Parent_C|SetMax%20AI%20Cars (Variables|/Game/Traffic_AI_System/Blueprints/BP_Traffic_path_50_Parent.BP_Traffic_path_50_Parent_C|GetMain%20Road _returnvalue) (+ (Variables|/Game/Traffic_AI_System/Blueprints/BP_Traffic_path_50_Parent.BP_Traffic_path_50_Parent_C|GetMax%20AI%20Cars (Variables|/Game/Traffic_AI_System/Blueprints/BP_Traffic_path_50_Parent.BP_Traffic_path_50_Parent_C|GetMain%20Road _returnvalue)) 1))))

(event Input|KeyboardEvents|Subtract
  (params (Key :type Key%20Structure :default "None"))
  ;[1 0.9353 0.4875] Inputs
  (:Pressed
    (bind _returnvalue (Actor|GetActorOfClass "/Game/Traffic_AI_System/Blueprints/BP_Traffic_path_50_Parent.BP_Traffic_path_50_Parent_C"))
    (Variables|/Game/Traffic_AI_System/Blueprints/BP_Traffic_path_50_Parent.BP_Traffic_path_50_Parent_C|SetMax%20AI%20Cars (Variables|/Game/Traffic_AI_System/Blueprints/BP_Traffic_path_50_Parent.BP_Traffic_path_50_Parent_C|GetMain%20Road _returnvalue) (+ (Variables|/Game/Traffic_AI_System/Blueprints/BP_Traffic_path_50_Parent.BP_Traffic_path_50_Parent_C|GetMax%20AI%20Cars (Variables|/Game/Traffic_AI_System/Blueprints/BP_Traffic_path_50_Parent.BP_Traffic_path_50_Parent_C|GetMain%20Road _returnvalue)) -1))))

(event Input|KeyboardEvents|Period
  (params (Key :type Key%20Structure :default "None"))
  ;[1 0.9353 0.4875] Inputs
  (:Pressed
    (bind _returnvalue (Actor|GetActorOfClass "/Game/Traffic_AI_System/Preview/Preview_blueprints/BP_Time_of_day_preview.BP_Time_of_day_preview_C"))
    (Variables|/Game/Traffic_AI_System/Preview/Preview_blueprints/BP_Time_of_day_preview.BP_Time_of_day_preview_C|SetTime%20of%20day _returnvalue (select (> (+ (Variables|/Game/Traffic_AI_System/Preview/Preview_blueprints/BP_Time_of_day_preview.BP_Time_of_day_preview_C|GetTime%20of%20day _returnvalue) 1.0) 24.0) (- (+ (Variables|/Game/Traffic_AI_System/Preview/Preview_blueprints/BP_Time_of_day_preview.BP_Time_of_day_preview_C|GetTime%20of%20day _returnvalue) 1.0) 24.0) (+ (Variables|/Game/Traffic_AI_System/Preview/Preview_blueprints/BP_Time_of_day_preview.BP_Time_of_day_preview_C|GetTime%20of%20day _returnvalue) 1.0)))))

(fn ConstructionScript)