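; Traffic signal actor that cycles its red, yellow, green left-turn and green lamps through up to four configurable phases, looping from BeginPlay.
; Macros Seq1 to Seq4 run in turn, each reading its own Sequence settings and passing straight on when Use is off.
; An active phase swaps BodyMesh lamp materials between ON and OFF, toggles the matching components' visibility, then delays for its duration before the next.
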(event EventBeginPlay
  (|Seq1 :!label _label
    (:then
      _)
    (:Not%20use
      _))
  (|Seq2
    (:then
      _)
    (:Not%20Use
      _))
  (|Seq3
    (:then
      _)
    (:Not%20Use
      _))
  (|Seq4
    (:then
      (goto _label))
    (:Not%20Use
      (goto _label))))

(event Collision|EventActorBeginOverlap
  (params (OtherActor :type Actor%20Object%20Reference)))

(event EventTick
  (params (DeltaSeconds :type Float%20%28single-precision%29)))

(fn ConstructionScript)