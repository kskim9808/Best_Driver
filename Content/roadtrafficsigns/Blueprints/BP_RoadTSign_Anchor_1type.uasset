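; Road traffic sign anchor Blueprint that builds a single sign when it is constructed.
; If the Sign1 struct is enabled, the construction script adds a static mesh component and picks its mesh from the Staticmeshes1 array by sign type.
; The mesh sits at a fixed raised offset with no rotation.
; The event graph holds only empty default events.
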(event EventBeginPlay)

(event Collision|EventActorBeginOverlap
  (params (OtherActor :type Actor%20Object%20Reference)))

(event EventTick
  (params (DeltaSeconds :type Float%20%28single-precision%29)))

(fn ConstructionScript
  (bind _sign_1 (Variables|SignSettings|GetSign%201))
  (bind (_use _signtype) (Utilities|Struct|BreakBiglsizeSign _sign_1))
  (if _use
    (bind _returnvalue (AddComponent|AddStaticMeshComponent false))
    (Components|StaticMesh|SetStaticMesh _returnvalue (Utilities|Array|Get(acopy) (Utilities|Struct|BreakBigSizeSignmesh (Variables|SignSettings|GetStaticmeshes1)) (Math|Conversions|ToInteger(Byte) _signtype)))
    (Transformation|SetRelativeLocationAndRotation _returnvalue (Math|Vector|RotateVectorAroundAxis (Math|Vector|MakeVector -0.5 0.0 45.0) 0.0 "0, 0,1.000000") "0,0.000000, 0" false false)))