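; Road traffic sign pole actor that assembles up to two configurable signs in its construction script, with no runtime logic.
; Each sign adds a mesh picked by sign type, placed by height and rotated around the pole.
; An optional description mesh sits below each sign with an extra half-turn.
; Sign 2 is skipped when Sign 1 is used without its description.
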(event EventBeginPlay)

(event Collision|EventActorBeginOverlap
  (params (OtherActor :type Actor%20Object%20Reference)))

(event EventTick
  (params (DeltaSeconds :type Float%20%28single-precision%29)))

(fn ConstructionScript
  (bind _sign_1 (Variables|SignSettings|GetSign%201))
  (bind _sign_2 (Variables|SignSettings|GetSign%202))
  (bind (_use _signtype _descriptiontextaffectspecificsigns _height _rotation) (Utilities|Struct|BreakNormalsizeSign _sign_1))
  (bind (_use_2 _signtype_2 _descriptiontextaffectspecificsigns_2 _height_2 _rotation_2) (Utilities|Struct|BreakNormalsizeSign _sign_2))
  (bind _returnvalue (Math|Conversions|ToInteger(Byte) _signtype))
  (bind _returnvalue_2 (Math|Conversions|ToFloat(Integer) _height))
  (bind _returnvalue_3 (Math|Conversions|ToFloat(Integer) _rotation))
  (bind _returnvalue_4 (Math|Conversions|ToInteger(Byte) _signtype_2))
  (bind _returnvalue_5 (Math|Conversions|ToFloat(Integer) _height_2))
  (bind _returnvalue_6 (Math|Conversions|ToFloat(Integer) _rotation_2))
  (if _use
    (bind _returnvalue_7 (AddComponent|AddStaticMeshComponent false))
    (Components|StaticMesh|SetStaticMesh _returnvalue_7 (Utilities|Array|Get(acopy) (Utilities|Struct|BreakNormalSizeSignmesh (Variables|SignSettings|GetStaticmeshes1)) _returnvalue))
    (Transformation|SetRelativeLocationAndRotation _returnvalue_7 (Math|Vector|RotateVectorAroundAxis (Math|Vector|MakeVector -3.5 0.0 _returnvalue_2) _returnvalue_3 "0, 0,1.000000") (Math|Rotator|MakeRotator 0.0 0.0 _returnvalue_3) false false)
    (if _descriptiontextaffectspecificsigns
      (bind _returnvalue_8 (AddComponent|AddStaticMeshComponent false))
      (Components|StaticMesh|SetStaticMesh _returnvalue_8 (Utilities|Array|Get(acopy) (Utilities|Struct|BreakNormalSizeSignText (Variables|SignSettings|GetDescTexts1)) _returnvalue))
      (Transformation|SetRelativeLocationAndRotation _returnvalue_8 (Math|Vector|RotateVectorAroundAxis (Math|Vector|MakeVector -3.5 0.0 (- _returnvalue_2 5e+01)) _returnvalue_3 "0, 0,1.000000") (Math|Rotator|MakeRotator 0.0 0.0 _returnvalue_3) false false)
      (Transformation|AddLocalRotation _returnvalue_8 "0,180.000000,0.000000" false false)
      (if _use_2 :!label _label
        (bind _returnvalue_9 (AddComponent|AddStaticMeshComponent false))
        (Components|StaticMesh|SetStaticMesh _returnvalue_9 (Utilities|Array|Get(acopy) (Utilities|Struct|BreakNormalSizeSignmesh (Variables|SignSettings|GetStaticmeshes2)) _returnvalue_4))
        (Transformation|SetRelativeLocationAndRotation _returnvalue_9 (Math|Vector|RotateVectorAroundAxis (Math|Vector|MakeVector -3.5 0.0 _returnvalue_5) _returnvalue_6 "0, 0,1.000000") (Math|Rotator|MakeRotator 0.0 0.0 _returnvalue_6) false false)
        (if _descriptiontextaffectspecificsigns_2
          (bind _returnvalue_10 (AddComponent|AddStaticMeshComponent false))
          (Components|StaticMesh|SetStaticMesh _returnvalue_10 (Utilities|Array|Get(acopy) (Utilities|Struct|BreakNormalSizeSignText (Variables|SignSettings|GetDescTexts2)) _returnvalue_4))
          (Transformation|SetRelativeLocationAndRotation _returnvalue_10 (Math|Vector|RotateVectorAroundAxis (Math|Vector|MakeVector -3.5 0.0 (- _returnvalue_5 5e+01)) _returnvalue_6 "0, 0,1.000000") (Math|Rotator|MakeRotator 0.0 0.0 _returnvalue_6) false false)
          (Transformation|AddLocalRotation _returnvalue_10 "0,180.000000,0.000000" false false))))
    (else
      (goto _label))))