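; Road traffic light controller that cycles three yellow lamps through up to ten configurable steps, looping endlessly from BeginPlay.
; Each Seq macro reads its Sequence settings, sets each lamp's on/off material and light visibility, then waits for the step's duration.
; Disabled steps are skipped without delay, so the loop has no wait if every step is disabled.
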(event EventBeginPlay
  (|Seq1 :!label _label
    (:then
      _)
    (:Not%20use
      _))
  (|Seq2
    (:then
      _)
    (:Not%20use
      _))
  (|Seq3
    (:then
      _)
    (:Not%20use
      _))
  (|Seq4
    (:then
      _)
    (:Not%20use
      _))
  (|Seq5
    (:then
      _)
    (:Not%20use
      _))
  (|Seq6
    (:then
      _)
    (:Not%20use
      _))
  (|Seq7
    (:then
      _)
    (:Not%20use
      _))
  (|Seq8
    (:then
      _)
    (:Not%20use
      _))
  (|Seq9
    (:then
      _)
    (:Not%20use
      _))
  (|Seq10
    (:then
      (goto _label))
    (:Not%20use
      (goto _label))))

(fn ConstructionScript)