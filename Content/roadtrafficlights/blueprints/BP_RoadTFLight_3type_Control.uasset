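; Road traffic light that cycles red, yellow, green left-turn arrow and green lamps through a timed, configurable program.
; BeginPlay chains ten near-identical collapsed graphs, Seq1 to Seq10, and loops back to the first.
; Each reads its SequenceN settings, skipping when Use is off, otherwise swapping mesh materials and toggling light visibility per lamp.
; The four lamp branches converge on one Delay of that step's duration before the next step runs.
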(event EventBeginPlay
  (|Seq1 :!label _label
    (:then
      _)
    (:Not%20use
      _))
  (|Seq2
    (:then
      _)
    (:Not%20Use
      _))
  (|Seq3
    (:then
      _)
    (:Not%20Use
      _))
  (|Seq4
    (:then
      _)
    (:Not%20Use
      _))
  (|Seq5
    (:then
      _)
    (:Not%20Use
      _))
  (|Seq6
    (:then
      _)
    (:Not%20Use
      _))
  (|Seq7
    (:then
      _)
    (:Not%20Use
      _))
  (|Seq8
    (:then
      _)
    (:Not%20Use
      _))
  (|Seq9
    (:then
      _)
    (:Not%20Use
      _))
  (|Seq10
    (:then
      (goto _label))
    (:Not%20Use
      (goto _label))))

(fn ConstructionScript)