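; Pedestrian traffic light that loops through up to five configurable red/green phases from BeginPlay.
; Seq1 to Seq5 are chained near-duplicate macros, each reading its Sequence struct and skipping when Use is off.
; Each phase swaps mesh materials, toggles light visibility and waits its duration, with optional green blinking through a DoN and Delay loop at one cycle per second.
; The construction script offsets Pin sideways based on LeftRight.
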(event EventBeginPlay
  (|Seq1 :!label _label
    (:then
      _)
    (:Not%20Use
      _))
  (|Seq2
    (:then
      _)
    (:Not%20Use
      _))
  (|Seq3
    (:then
      _)
    (:Not%20Use
      _))
  (|Seq4
    (:then
      _)
    (:Not%20Use
      _))
  (|Seq5
    (:then
      (goto _label))
    (:Not%20Use
      (goto _label))))

(fn ConstructionScript
  (if (Variables|PinDirection|GetLeft%20/%20Right)
    (bind _output_get (Variables|SignalSettings|SetPin (Variables|SignalSettings|GetPin)))
    (Transformation|SetRelativeTransform _output_get (Math|Transform|MakeTransform "7.000000,-25.000000,0.000000") false false)
    (else
      (bind _output_get_2 (Variables|SignalSettings|SetPin (Variables|SignalSettings|GetPin)))
      (Transformation|SetRelativeTransform _output_get_2 (Math|Transform|MakeTransform "7.000000,25.000000,0.000000") false false))))